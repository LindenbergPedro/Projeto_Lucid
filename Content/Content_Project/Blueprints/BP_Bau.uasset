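; BP_Bau is a chest actor that opens and closes automatically based on the player's proximity.
; Begin and end overlap events on its Collision_Bau component cast the other actor to BP_CHARACTER, then call the Abrir (open) or Fechar (close) custom event.
; Each event instantly sets the TopoBau lid's relative rotation, with no animation or interpolation.
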(event `self.Collision_Bau.OnComponentBeginOverlap`
  (params (OverlappedComponent :type "PrimitiveComponent Object Reference") (OtherActor :type "Actor Object Reference") (OtherComp :type "PrimitiveComponent Object Reference") (OtherBodyIndex :type Integer) (bFromSweep :type Boolean) (SweepResult :type "HitResult Structure (by ref)"))
  ;[1 1 1] Verificação de Overlap do Bau.
  (cast `/Game/Content_Project/Blueprints/Character/BP_CHARACTER` OtherActor)
  (`self.Abrir`))

(event `self.Collision_Bau.OnComponentEndOverlap`
  (params (OverlappedComponent :type "PrimitiveComponent Object Reference") (OtherActor :type "Actor Object Reference") (OtherComp :type "PrimitiveComponent Object Reference") (OtherBodyIndex :type Integer))
  ;[1 1 1] Verificação de Overlap do Bau.
  (cast `/Game/Content_Project/Blueprints/Character/BP_CHARACTER` OtherActor)
  (`self.Fechar`))

(event `Abrir`
  (`SceneComponent.K2_SetRelativeRotation` (`self.Topo_Bau`) (struct :`Pitch` 90.0) false false))

(event `Fechar`
  (`SceneComponent.K2_SetRelativeRotation` (`self.Topo_Bau`) (struct) false false))

(fn `UserConstructionScript`)