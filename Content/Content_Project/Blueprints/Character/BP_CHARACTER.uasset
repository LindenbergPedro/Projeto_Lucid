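; Player character with world-axis movement, jumping and object pushing, viewed through a separate BP_CameraFollow actor.
; The follow actor interpolates toward the character's spring-arm camera each tick, while Left/Right keys shift the arm sideways and quicken the interpolation.
; Interact searches a debug-drawn sphere at the feet and messages the first InteractInterface actor, or ends an active push.
; BPPushComponent's pushing state blocks normal movement and jumping.
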(event `self.ReceiveBeginPlay`
  (bind _outactors (`GameplayStatics.GetAllActorsOfClass` "/Game/Content_Project/Blueprints/Camera/BP_CameraFollow.BP_CameraFollow_C"))
  (set `self.ActiveCamera` (`|GetArrayItem` _outactors))
  (`PlayerController.SetViewTargetWithBlend` (`GameplayStatics.GetPlayerController` 0) (`self.ActiveCamera`) 0.0 "VTBlend_Linear" 0.0 false)
  (`self.K2_SetActorLocation` (`self.ActiveCamera`) (`SceneComponent.K2_GetComponentLocation` (`self.Camera`)) false false))

(event `self.ReceiveTick`
  (params (DeltaSeconds :type "Float (single-precision)"))
  (`self.K2_SetActorLocation` (`self.ActiveCamera`) (`KismetMathLibrary.VInterpTo` (`self.K2_GetActorLocation` (`self.ActiveCamera`)) (`SceneComponent.K2_GetComponentLocation` (`self.Camera`)) (`GameplayStatics.GetWorldDeltaSeconds`) (`self. Interpsspeed`)) false false))

(event `InputAxis|MoveRight`
  (params (AxisValue :type "Float (single-precision)"))
  (if (not (`/Game/Content_Project/Blueprints/Pushable/BP_pushComponent.IsPushingObject` (`self.BP_pushComponent`)))
    (`self.AddMovementInput` (0.0 1.0 0.0) AxisValue)))

(event `InputAxis|MoveForward`
  (params (AxisValue :type "Float (single-precision)"))
  (if (not (`/Game/Content_Project/Blueprints/Pushable/BP_pushComponent.IsPushingObject` (`self.BP_pushComponent`)))
    (`self.AddMovementInput` (1.0 0.0 0.0) AxisValue)))

(event `InputAction|Jump`
  (params (Key :type "Key Structure"))
  (:`Pressed`
    (if (not (`/Game/Content_Project/Blueprints/Pushable/BP_pushComponent.IsPushingObject` (`self.BP_pushComponent`)))
      (`self.Jump`)))
  (:`Released`
    (`self.StopJumping`)))

(event `Key|Right`
  (params (Key :type "Key Structure"))
  (bind _springarm (`self.SpringArm`))
  (:`Pressed`
    (set `SpringArmComponent.TargetOffset` (0.0 200.0 0.0) _springarm)
    (set `self. Interpsspeed` 2.5))
  (:`Released`
    (set `SpringArmComponent.TargetOffset` (0.0 0.0 0.0) _springarm)
    (set `self. Interpsspeed` 1.5)))

(event `Key|Left`
  (params (Key :type "Key Structure"))
  (bind _springarm (`self.SpringArm`))
  (:`Pressed`
    (set `SpringArmComponent.TargetOffset` (0.0 -200.0 0.0) _springarm)
    (set `self. Interpsspeed` 2.5))
  (:`Released`
    (set `SpringArmComponent.TargetOffset` (0.0 0.0 0.0) _springarm)
    (set `self. Interpsspeed` 1.5)))

(event `InputAction|Interact`
  (params (Key :type "Key Structure"))
  ;[1 1 1] Pushing
  (:`Pressed`
    (if (not (`/Game/Content_Project/Blueprints/Pushable/BP_pushComponent.IsPushingObject` (`self.BP_pushComponent`)))
      (bind _outactors (`self.SphereOverlapActors` (- (`self.K2_GetActorLocation`) (`KismetMathLibrary.MakeVector` 0.0 0.0 (`CapsuleComponent.GetScaledCapsuleHalfHeight` (`self.CapsuleComponent`)))) (`/Game/Content_Project/Blueprints/Pushable/BP_pushComponent.PushRange` (`self.BP_pushComponent`))))
      (for _array_element _outactors
        (if (`KismetSystemLibrary.DoesImplementInterface` _array_element "/Game/Content_Project/Blueprints/InteractInterface.InteractInterface_C")
          (message `/Game/Content_Project/Blueprints/InteractInterface.OnInteracted` _array_element self)
          (break)))
      (else
        (`/Game/Content_Project/Blueprints/Pushable/BP_pushComponent.EndPush` (`self.BP_pushComponent`))))))

(fn `AfastaSpring`
  (params (TargetArmLength :type "Float (double-precision)"))
  (set `SpringArmComponent.TargetArmLength` TargetArmLength (`self.SpringArm`)))

(fn `SphereOverlapActors`
  (params (Center :type "Vector Structure") (Radius :type "Float (double-precision)"))
  (returns (OutActors :type "Array of Actor Object Reference"))
  (`|ExecutionSequence`
    (:`then_0`
      (`KismetSystemLibrary.DrawDebugSphere` (`local.Center`) (`local.Radius`) 12 (struct :`R` 1.0 :`G` 1.0 :`B` 1.0 :`A` 1.0) 2.0 1.0))
    (:`then_1`
      (bind _outactors (`KismetSystemLibrary.SphereOverlapActors` (`local.Center`) (`local.Radius`) (`|MakeArray` "ObjectTypeQuery2" :!type "EObjectTypeQuery Enum") null (`|MakeArray` self :!type "Actor Object Reference")))
      (return _outactors))))

(fn `UserConstructionScript`)

(fn `VoltaSpring`
  (set `SpringArmComponent.TargetArmLength` 450.0 (`self.SpringArm`)))